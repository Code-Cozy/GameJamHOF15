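; PC_Nano is the player controller for an Articy-driven visual novel, creating the switcher UI and handling input, pausing and game start and end.
; Articy flow player events push dialogue text and speaker sprites to the HUD, then rebuild choice widgets, adding a close widget when none exist.
; Sprites and backgrounds come from name-keyed data tables.
; String-argument functions set backgrounds and play named sound effects.
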(event OnPlayerPaused(ArticyFlowPlayer)
  (params (PausedOn :type Articy%20Flow%20Object%20Interface))
  ;[0.15 0.15 0.15 0.5] play dialogue
  (bind _output_get (Variables|Default|SetCurrent%20Branch PausedOn))
  (bind _asarticy_node (Utilities|Casting|CastToArticyNode _output_get))
  (switch Utilities|FlowControl|Switch|SwitchonEArticyPausableType (Class|ArticyNode|GetType _asarticy_node)
    (:Dialogue
      (Class|ArticyFlowPlayer|Play (Variables|Default|GetArticyFlowPlayer)))
    (:DialogueFragment
      (bind _asarticy_object_with_text (Utilities|Casting|CastToArticyObjectWithText (Variables|Default|GetCurrent%20Branch)))
      (bind _returnvalue (Class|ArticyObjectwithText|GetText _asarticy_object_with_text))
      (Default|UpdateDialogueText (Variables|Default|GetWidget) _returnvalue)
      (bind _asarticy_object_with_speaker (Utilities|Casting|CastToArticyObjectWithSpeaker (Variables|Default|GetCurrent%20Branch)))
      (bind _asnanoreno_default_main_character_template (Utilities|Casting|CastToNanorenoDefaultMainCharacterTemplate (Class|ArticyObjectwithSpeaker|GetSpeaker _asarticy_object_with_speaker)))
      (bind _returnvalue_2 (Class|ArticyObjectwithDisplayName|GetDisplayName _asnanoreno_default_main_character_template))
      (bind _returnvalue_3 (Utilities|GetDataTableRow "/Game/Blueprints/DT_Sprites.DT_Sprites" (Utilities|String|StringToName (Utilities|String|ToString(Text) _returnvalue_2)))
        (:then
          (Utilities|IsValid (Utilities|Array|Get(acopy) (.sprites _returnvalue_3))
            (:Is%20Valid
              (Default|UpdateSpeaker (Variables|/Game/Widgets/WBP_Switcher.WBP_Switcher_C|GetWBP_HUD (Variables|Default|GetWidget)) (Utilities|Array|Get(acopy) (.sprites _returnvalue_3))))
            (:Is%20Not%20Valid
              (Development|PrintString "Character Does Not Have Sprite!"))))
        (:RowNotFound
          (Development|PrintString "Character Does Not Exist!"))))))

(event OnBranchesUpdated(ArticyFlowPlayer)
  (params (AvailableBranches :type Array%20of%20Articy%20Branch%20Structures))
  ;[0.15 0.15 0.15 0.5] Update options
  (Variables|Default|SetHas%20Options? false)
  (Default|RemoveOptions (Variables|Default|GetWidget))
  (for _array_element AvailableBranches
    (Utilities|Casting|CastToArticyObjectWithText (Class|ArticyFunctionLibrary|GetBranchTarget _array_element))
    (bind _returnvalue (UserInterface|CreateWidget "/Game/Widgets/WBP_Advance.WBP_Advance_C" 0 (Variables|Default|GetArticyFlowPlayer) _array_element))
    (Default|AddOption (Variables|Default|GetWidget) _returnvalue)
    (Variables|Default|SetHas%20Options? true))
  (if (not (Variables|Default|GetHas%20Options?))
    (bind _returnvalue_2 (UserInterface|CreateWidget "/Game/Widgets/WBP_Close.WBP_Close_C"))
    (Default|AddOption (Variables|Default|GetWidget) _returnvalue_2)))

(event Custom|Start%20Dialouge
  ;[0.15 0.15 0.15 0.5] Start Game
  (Class|ArticyFlowPlayer|Play (Variables|Default|GetArticyFlowPlayer) -1)
  (Default|SwitchWidget (Variables|Default|GetWidget) 1))

(event Custom|End%20Dialouge
  ;[0.15 0.15 0.15 0.5] play dialogue
  (Game|QuitGame 0 "Quit" false))

(event Custom|Update%20Screen
  (params (Active%20Widget%20Index :type Integer))
  ;[0.15 0.15 0.15 0.5] Switch widget index
  (Default|SwitchWidget (Variables|Default|GetWidget) Active%20Widget%20Index))

(event Input|EnhancedActionEvents|EnhancedInputActionIA_Pause
  (params (ActionValue :type Boolean) (ElapsedSeconds :type Float%20%28double-precision%29) (TriggeredSeconds :type Float%20%28double-precision%29) (InputAction :type Input%20Action%20Object%20Reference :default "/Game/Blueprints/IA_Pause.IA_Pause"))
  (bind _widget (Variables|Default|GetWidget))
  (:Started
    (if (not (Variables|/Game/Widgets/WBP_Switcher.WBP_Switcher_C|GetMenu _widget))
      (if (Variables|/Game/Widgets/WBP_Switcher.WBP_Switcher_C|GetPaused _widget)
        (Default|SwitchWidget (Variables|Default|GetWidget) 1)
        (else
          (Default|SwitchWidget (Variables|Default|GetWidget) 2))))))

(event EventBeginPlay
  (bind _self self)
  (bind _returnvalue (PlayerController|LocalPlayerSubsystems|GetEnhancedInputLocalPlayerSubsystem _self))
  ;[0.15 0.15 0.15 0.5] spawn menu and, update input, show cursor
  (bind _returnvalue_2 (UserInterface|CreateWidget "/Game/Widgets/WBP_Switcher.WBP_Switcher_C"))
  (bind _output_get (Variables|Default|SetWidget _returnvalue_2))
  (UserInterface|Viewport|AddtoPlayerScreen _output_get)
  (Input|SetInputModeGameandUI self _output_get "DoNotLock" false false)
  (Variables|Default|SetbShowMouseCursor true)
  (Utilities|IsValid _returnvalue
    (:Is%20Valid
      (Input|AddMappingContext _returnvalue "/Game/Blueprints/IMC_Nano.IMC_Nano" 0 "(bIgnoreAllPressedKeysUntilRelease=True,bForceImmediately=False,bNotifyUserSettings=False)"))))

(fn ConstructionScript)

(fn PlaySoundString
  (params (aParam0 :type String))
  (switch string aParam0
    (:Loud%20Crash%20from%20Above
      (Audio|PlaySound2D "/Game/Sounds/20809__freqman__crash14-pot-back-in-cupboard.20809__freqman__crash14-pot-back-in-cupboard" 1.0 1.0 0.0 0 0))
    (:Thwack
      (Audio|PlaySound2D "/Game/Sounds/240980__dheming__wood_chop_01.240980__dheming__wood_chop_01" 1.0 1.0 0.0 0 0))
    (:Knock%20Knock
      (Audio|PlaySound2D "/Game/Sounds/182041__waveadventurer__five_sharp_knocks_on_computer_room_door.182041__waveadventurer__five_sharp_knocks_on_computer_room_door" 1.0 1.0 0.0 0 0)))
  (return false))

(fn SetBackgroundString
  (params (aParam0 :type String))
  (bind _returnvalue (Utilities|GetDataTableRow "/Game/Blueprints/DT_Backgrounds.DT_Backgrounds" (Utilities|String|StringToName aParam0))
    (:then
      (Utilities|IsValid (.image _returnvalue)
        (:Is%20Valid
          (Default|UpdateBackground (Variables|/Game/Widgets/WBP_Switcher.WBP_Switcher_C|GetWBP_HUD (Variables|Default|GetWidget)) (.image _returnvalue))
          (return true))
        (:Is%20Not%20Valid
          (Development|PrintString "Location Does Not Have Background!"))))
    (:RowNotFound
      (Development|PrintString "Location Does Not Exist!"))))