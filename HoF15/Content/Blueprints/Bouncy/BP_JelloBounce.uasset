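; BP_JelloBounce is a jello bounce pad that stays hidden and non-colliding until a Jello event activates it.
; On BeginPlay it disables itself and binds to the Jelloo event, which shows the mesh and enables the box collision.
; When the player character overlaps the box, it is launched with an overridden vertical velocity and a pitch-randomized bloop sound plays.
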(event OnComponentBeginOverlap(Box)
  (params (OverlappedComponent :type Primitive%20Component%20Object%20Reference) (OtherActor :type Actor%20Object%20Reference) (OtherComp :type Primitive%20Component%20Object%20Reference) (OtherBodyIndex :type Integer) (bFromSweep :type Boolean) (SweepResult :type Hit%20Result%20Structure%20%28by%20ref%29))
  ;[0 1 1] launch character
  (if (== OtherActor (Game|GetPlayerCharacter 0))
    (Character|LaunchCharacter (Game|GetPlayerCharacter 0) (Variables|Default|GetLaunch%20Velocity) false true)
    (Audio|PlaySound2D "/Game/Sound/S_bloop.S_bloop" 1.0 (Math|Random|RandomFloatinRange 0.8 1.2) 0.0 0 0)))

(event Custom|JEllo
  (Collision|SetCollisionEnabled (Variables|Default|GetBox) "QueryAndPhysics")
  (Rendering|SetVisibility (Variables|Default|GetStaticMesh) true false))

(event EventBeginPlay
  (Collision|SetCollisionEnabled (Variables|Default|GetBox) "NoCollision")
  (Rendering|SetVisibility (Variables|Default|GetStaticMesh) false false)
  (EventDispatchers|BindEventtoJelloo (delegate Custom|JEllo)))

(fn ConstructionScript)