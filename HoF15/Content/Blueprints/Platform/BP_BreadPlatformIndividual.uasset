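; An individual bread platform that starts hidden and non-collidable while shuttling endlessly between its start and end points.
; A timeline lerps the mesh with teleporting moves and reverses on each finish, its play rate being the inverse of MovementSpeed.
; The Platform event, bound to PlatformPlease at BeginPlay, reveals the mesh and enables collision after a short delay.
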(event Custom|Movment%20Backward
  (bind (_direction _move_it) (Timeline|Timeline ReverseFromEnd)
    (:Update
      (Transformation|SetWorldLocation (Variables|Default|GetStaticMesh) (Math|Vector|Lerp(Vector) (Transformation|GetWorldLocation (Variables|Default|GetStartPoint)) (Transformation|GetWorldLocation (Variables|Default|GetEndPoint)) _move_it) false true))
    (:Finished
      (switch Utilities|FlowControl|Switch|SwitchonETimelineDirection _direction
        (:Forward
          (CallFunction|MovmentBackward))
        (:Backward
          (CallFunction|MovementForward))))))

(event Custom|Movement%20Forward
  (bind (_direction _move_it) (Timeline|Timeline PlayFromStart)
    (:Update
      (Transformation|SetWorldLocation (Variables|Default|GetStaticMesh) (Math|Vector|Lerp(Vector) (Transformation|GetWorldLocation (Variables|Default|GetStartPoint)) (Transformation|GetWorldLocation (Variables|Default|GetEndPoint)) _move_it) false true))
    (:Finished
      (switch Utilities|FlowControl|Switch|SwitchonETimelineDirection _direction
        (:Forward
          (CallFunction|MovmentBackward))
        (:Backward
          (CallFunction|MovementForward))))))

(event Custom|Platform
  (Utilities|FlowControl|Delay 0.2)
  (Collision|SetCollisionEnabled (Variables|Default|GetStaticMesh) "QueryAndPhysics")
  (Rendering|SetVisibility (Variables|Default|GetStaticMesh) true false))

(event EventBeginPlay
  (Collision|SetCollisionEnabled (Variables|Default|GetStaticMesh) "NoCollision")
  (Rendering|SetVisibility (Variables|Default|GetStaticMesh) false false)
  (EventDispatchers|BindEventtoPlatformPlease (delegate Custom|Platform))
  (Components|Timeline|SetPlayRate (Variables|Default|GetTimeline) (/ 1.0 (Variables|Default|GetMovement%20Speed)))
  (CallFunction|MovementForward))

(fn ConstructionScript)