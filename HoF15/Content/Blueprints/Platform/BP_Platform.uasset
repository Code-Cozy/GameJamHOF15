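; BP_Platform is a moving platform that shuttles its static mesh back and forth between StartPoint and EndPoint, starting at BeginPlay.
; A timeline drives a linear interpolation between the world locations of the two points, setting the mesh position with teleport and no sweep.
; When the timeline finishes, its direction selects either a reverse or a forward replay, creating an endless ping-pong loop.
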(event Custom|Movment%20Backward
  (bind (_direction _move_it) (Timeline|Timeline ReverseFromEnd)
    (:Update
      (Transformation|SetWorldLocation (Variables|Default|GetStaticMesh) (Math|Vector|Lerp(Vector) (Transformation|GetWorldLocation (Variables|Default|GetStartPoint)) (Transformation|GetWorldLocation (Variables|Default|GetEndPoint)) _move_it) false true))
    (:Finished
      (switch Utilities|FlowControl|Switch|SwitchonETimelineDirection _direction
        (:Forward
          (CallFunction|MovmentBackward))
        (:Backward
          (CallFunction|MovementForward))))))

(event Custom|Movement%20Forward
  (bind (_direction _move_it) (Timeline|Timeline PlayFromStart)
    (:Update
      (Transformation|SetWorldLocation (Variables|Default|GetStaticMesh) (Math|Vector|Lerp(Vector) (Transformation|GetWorldLocation (Variables|Default|GetStartPoint)) (Transformation|GetWorldLocation (Variables|Default|GetEndPoint)) _move_it) false true))
    (:Finished
      (switch Utilities|FlowControl|Switch|SwitchonETimelineDirection _direction
        (:Forward
          (CallFunction|MovmentBackward))
        (:Backward
          (CallFunction|MovementForward))))))

(event EventBeginPlay
  (CallFunction|MovementForward))

(fn ConstructionScript)