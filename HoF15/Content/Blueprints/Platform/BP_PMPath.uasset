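; BP_PMPath is a platform Blueprint that moves its static mesh from a start point to an end point when a Raise event fires.
; BeginPlay binds the Raise handler, which sets the timeline play rate to the inverse of MovementSpeed and starts forward movement.
; The timeline lerps world location with teleport and no sweep, restarting on finish only if its direction is Backward.
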(event Custom|Movement%20Forward
  (bind (_direction _move_it) (Timeline|Timeline PlayFromStart)
    (:Update
      (Transformation|SetWorldLocation (Variables|Default|GetStaticMesh) (Math|Vector|Lerp(Vector) (Transformation|GetWorldLocation (Variables|Default|GetStartPoint)) (Transformation|GetWorldLocation (Variables|Default|GetEndPoint)) _move_it) false true))
    (:Finished
      (switch Utilities|FlowControl|Switch|SwitchonETimelineDirection _direction
        (:Backward
          (CallFunction|MovementForward))))))

(event Custom|Raise_Event
  (if true
    (Components|Timeline|SetPlayRate (Variables|Default|GetTimeline) (/ 1.0 (Variables|Default|GetMovement%20Speed)))
    (CallFunction|MovementForward)))

(event EventBeginPlay
  (EventDispatchers|BindEventtoRaise (delegate Custom|Raise_Event)))

(fn ConstructionScript)