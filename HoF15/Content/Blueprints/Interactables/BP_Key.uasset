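; BP_Key is an interactable key pickup with a floating name prompt.
; An overlap radius shows or hides the WBP_Interact widget and updates the player's current interactable message.
; While the player is in range, Tick yaws the widget toward the player's mesh.
; Interact, noted as overridable by children, passes an Int to the player's GetKeyMessage, plays a randomly pitched sound, and destroys the key.
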(event OnComponentBeginOverlap(InteractRadius)
  (params (OverlappedComponent :type Primitive%20Component%20Object%20Reference) (OtherActor :type Actor%20Object%20Reference) (OtherComp :type Primitive%20Component%20Object%20Reference) (OtherBodyIndex :type Integer) (bFromSweep :type Boolean) (SweepResult :type Hit%20Result%20Structure%20%28by%20ref%29))
  ;[0 1 1] widget logic
  (if (== OtherActor (Game|GetPlayerCharacter 0))
    (Variables|Default|SetInteracting? true)
    (Variables|/Script/UMG.Widget|SetRenderOpacity (Variables|Components|GetMy%20Widget) 1.0)
    (Class|BPIPlayer|UpdateInteractable(Message) (Game|GetPlayerCharacter 0) self)))

(event OnComponentEndOverlap(InteractRadius)
  (params (OverlappedComponent :type Primitive%20Component%20Object%20Reference) (OtherActor :type Actor%20Object%20Reference) (OtherComp :type Primitive%20Component%20Object%20Reference) (OtherBodyIndex :type Integer))
  ;[0 1 1] widget logic
  (if (== (Game|GetPlayerCharacter 0) OtherActor)
    (Variables|Default|SetInteracting? false)
    (Variables|/Script/UMG.Widget|SetRenderOpacity (Variables|Components|GetMy%20Widget) 0.0)
    (Class|BPIPlayer|UpdateInteractable(Message) (Game|GetPlayerCharacter 0))))

(event EventBeginPlay
  ;[0 1 1] set up widget
  (bind _aswbp_interact (Utilities|Casting|CastToWBP_Interact (UserInterface|GetWidget (Variables|Default|GetWidget))))
  (bind _output_get (Variables|Components|SetMy%20Widget _aswbp_interact))
  (Variables|/Game/Widget/WBP_Interact.WBP_Interact_C|SetInteractable%20Name _output_get (Variables|Default|GetDisplay%20Name))
  (Variables|/Script/UMG.Widget|SetRenderOpacity _output_get 0.0))

(event EventTick
  (params (DeltaSeconds :type Float%20%28single-precision%29))
  ;[0 1 1] update widget rotation if you are interacting
  (if (Variables|Default|GetInteracting?)
    (Transformation|SetWorldRotation (Variables|Default|GetWidget) (Math|Rotator|MakeRotator 0.0 0.0 (.yaw (Math|Rotator|FindLookatRotation (Transformation|GetWorldLocation (Variables|Default|GetWidget)) (Transformation|GetWorldLocation (Variables|/Script/Engine.Character|GetMesh (Game|GetPlayerCharacter 0)))))) false false)))

(event EventInteract
  ;[0 1 1] simple interact event, can be changed for children
  (Class|BPIPlayer|GetKey(Message) (Game|GetPlayerCharacter 0) (Variables|Default|GetInt))
  (Audio|PlaySound2D "/Game/Sound/S_bloop_hover_3_.S_bloop_hover_3_" 1.0 (Math|Random|RandomFloatinRange 0.8 1.2) 0.0 0 0)
  (Actor|DestroyActor))

(fn ConstructionScript)