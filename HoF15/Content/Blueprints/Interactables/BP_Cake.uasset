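; BP_Cake is an interactable cake that flees along a spline when first interacted with, then can be eaten with a sound and destroyed once it stops.
; A Before/During/After state gates interaction and the player-facing prompt widget, which appears within InteractRadius.
; A timeline scaled by Playrate moves the skeletal mesh along the spline.
; Straying too far from the actor during the run opens the menu map.
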(event OnComponentBeginOverlap(InteractRadius)
  (params (OverlappedComponent :type Primitive%20Component%20Object%20Reference) (OtherActor :type Actor%20Object%20Reference) (OtherComp :type Primitive%20Component%20Object%20Reference) (OtherBodyIndex :type Integer) (bFromSweep :type Boolean) (SweepResult :type Hit%20Result%20Structure%20%28by%20ref%29))
  ;[0 1 1] widget logic
  (if (== OtherActor (Game|GetPlayerCharacter 0))
    (switch Utilities|FlowControl|Switch|SwitchonE_Trial (Variables|Default|GetState)
      (:NewEnumerator0
        _)
      (:NewEnumerator2
        _))
    (Variables|Default|SetInteracting? true)
    (Variables|/Script/UMG.Widget|SetRenderOpacity (Variables|Components|GetMy%20Widget) 1.0)
    (Class|BPIPlayer|UpdateInteractable(Message) (Game|GetPlayerCharacter 0) self)))

(event OnComponentEndOverlap(InteractRadius)
  (params (OverlappedComponent :type Primitive%20Component%20Object%20Reference) (OtherActor :type Actor%20Object%20Reference) (OtherComp :type Primitive%20Component%20Object%20Reference) (OtherBodyIndex :type Integer))
  ;[0 1 1] widget logic
  (if (== (Game|GetPlayerCharacter 0) OtherActor)
    (switch Utilities|FlowControl|Switch|SwitchonE_Trial (Variables|Default|GetState)
      (:NewEnumerator0
        _)
      (:NewEnumerator2
        _))
    (Variables|Default|SetInteracting? false)
    (Variables|/Script/UMG.Widget|SetRenderOpacity (Variables|Components|GetMy%20Widget) 0.0)
    (Class|BPIPlayer|UpdateInteractable(Message) (Game|GetPlayerCharacter 0))))

(event Custom|Run
  (bind _spline (Variables|Default|GetSpline))
  ;[0 1 1] movement of cake
  (bind _movement (Timeline|Timeline PlayFromStart)
    (:Update
      (Transformation|SetWorldLocation (Variables|Default|GetSkeletalMesh) (Spline|GetLocationatDistanceAlongSpline (Variables|Default|GetSpline) (Math|Float|Lerp 0.0 (Spline|GetDistanceAlongSplineatSplinePoint _spline (- (Spline|GetNumberOfSplinePoints _spline) 1)) _movement) "World") false true))
    (:Finished
      (Variables|Default|SetState "NewEnumerator2")
      (if (Collision|IsOverlappingActor (Variables|Default|GetInteract%20Radius) (Game|GetPlayerCharacter 0) :!class /Script/Engine.PrimitiveComponent)
        (CallFunction|Turnon)))))

(event Custom|Turn%20Off
  ;[0 1 1] widget logic
  (Variables|Default|SetInteracting? false)
  (Variables|/Script/UMG.Widget|SetRenderOpacity (Variables|Components|GetMy%20Widget) 0.0)
  (Class|BPIPlayer|UpdateInteractable(Message) (Game|GetPlayerCharacter 0)))

(event Custom|Turn%20On
  ;[0 1 1] widget logic
  (Variables|Default|SetInteracting? true)
  (Variables|/Script/UMG.Widget|SetRenderOpacity (Variables|Components|GetMy%20Widget) 1.0)
  (Class|BPIPlayer|UpdateInteractable(Message) (Game|GetPlayerCharacter 0) self))

(event EventBeginPlay
  ;[0 1 1] set up widget
  (bind _aswbp_interact (Utilities|Casting|CastToWBP_Interact (UserInterface|GetWidget (Variables|Default|GetWidget))))
  (bind _output_get (Variables|Components|SetMy%20Widget _aswbp_interact))
  (Variables|/Game/Widget/WBP_Interact.WBP_Interact_C|SetInteractable%20Name _output_get (Variables|Default|GetDisplay%20Name))
  (Variables|/Script/UMG.Widget|SetRenderOpacity _output_get 0.0)
  ;[0 1 1] set speed of movement on timeline
  (Components|Timeline|SetPlayRate (Variables|Default|GetTimeline) (/ 1.0 (Variables|Default|GetPlayrate))))

(event EventInteract
  ;[0 1 1] simple interact event, can be changed for children
  (switch Utilities|FlowControl|Switch|SwitchonE_Trial (Variables|Default|GetState)
    (:NewEnumerator0
      (Variables|Default|SetState "NewEnumerator1")
      (CallFunction|Run)
      (CallFunction|TurnOff))
    (:NewEnumerator2
      (Audio|PlaySound2D "/Game/Sound/S_yumyum.S_yumyum" 1.0 1.0 0.0 0 0)
      (Actor|DestroyActor))))

(event EventTick
  (params (DeltaSeconds :type Float%20%28single-precision%29))
  ;[0 1 1] update widget rotation if you are interacting
  (switch Utilities|FlowControl|Switch|SwitchonE_Trial (Variables|Default|GetState)
    (:NewEnumerator0
      (if (Variables|Default|GetInteracting?) :!label _label
        (Transformation|SetWorldRotation (Variables|Default|GetWidget) (Math|Rotator|MakeRotator 0.0 0.0 (.yaw (Math|Rotator|FindLookatRotation (Transformation|GetWorldLocation (Variables|Default|GetWidget)) (Transformation|GetWorldLocation (Variables|/Script/Engine.Character|GetMesh (Game|GetPlayerCharacter 0)))))) false false)))
    (:NewEnumerator1
      (if (>= (Transformation|GetDistanceTo (Game|GetPlayerCharacter 0) self) 5e+03)
        (Game|OpenLevel(byObjectReference) "/Game/Maps/Map_Menu.Map_Menu")))
    (:NewEnumerator2
      (goto _label))))

(fn ConstructionScript)