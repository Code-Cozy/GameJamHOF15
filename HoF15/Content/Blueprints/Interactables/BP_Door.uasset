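; Interactable door that swings a hinge 90 degrees open or closed when its Interact event fires, meant as a base that children can change.
; An overlap radius registers it with the player character and shows two prompt widgets, "Open Door" and "Close Door", clearing both on exit.
; Interact plays a pitch-randomized sound, flips Open, then plays or reverses a timeline lerping hinge yaw from its starting value.
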(event OnComponentBeginOverlap(InteractRadius)
  (params (OverlappedComponent :type Primitive%20Component%20Object%20Reference) (OtherActor :type Actor%20Object%20Reference) (OtherComp :type Primitive%20Component%20Object%20Reference) (OtherBodyIndex :type Integer) (bFromSweep :type Boolean) (SweepResult :type Hit%20Result%20Structure%20%28by%20ref%29))
  ;[0 1 1] widget logic
  (if (== OtherActor (Game|GetPlayerCharacter 0))
    (Variables|Default|SetInteracting? true)
    (Variables|/Script/UMG.Widget|SetRenderOpacity (Variables|Components|GetMy%20Widget) 1.0)
    (Class|BPIPlayer|UpdateInteractable(Message) (Game|GetPlayerCharacter 0) self)
    (Variables|/Script/UMG.Widget|SetRenderOpacity (Variables|Components|GetMy%20Widget2) 1.0)))

(event OnComponentEndOverlap(InteractRadius)
  (params (OverlappedComponent :type Primitive%20Component%20Object%20Reference) (OtherActor :type Actor%20Object%20Reference) (OtherComp :type Primitive%20Component%20Object%20Reference) (OtherBodyIndex :type Integer))
  ;[0 1 1] widget logic
  (if (== (Game|GetPlayerCharacter 0) OtherActor)
    (Variables|Default|SetInteracting? false)
    (Variables|/Script/UMG.Widget|SetRenderOpacity (Variables|Components|GetMy%20Widget) 0.0)
    (Class|BPIPlayer|UpdateInteractable(Message) (Game|GetPlayerCharacter 0))
    (Variables|/Script/UMG.Widget|SetRenderOpacity (Variables|Components|GetMy%20Widget2) 0.0)))

(event EventBeginPlay
  ;[0 1 1] set up widget
  (Variables|Default|SetStart%20Z (.yaw (Transformation|GetWorldRotation (Variables|Default|GetHinge))))
  (Utilities|FlowControl|Sequence
    (:then_0
      (bind _aswbp_interact (Utilities|Casting|CastToWBP_Interact (UserInterface|GetWidget (Variables|Default|GetWidget))))
      (bind _output_get (Variables|Components|SetMy%20Widget _aswbp_interact))
      (Variables|/Game/Widget/WBP_Interact.WBP_Interact_C|SetInteractable%20Name _output_get "Open Door")
      (Variables|/Script/UMG.Widget|SetRenderOpacity _output_get 0.0))
    (:then_1
      (bind _aswbp_interact_2 (Utilities|Casting|CastToWBP_Interact (UserInterface|GetWidget (Variables|Default|GetWidget1))))
      (bind _output_get_2 (Variables|Components|SetMy%20Widget2 _aswbp_interact_2))
      (Variables|/Game/Widget/WBP_Interact.WBP_Interact_C|SetInteractable%20Name _output_get_2 "Close Door")
      (Variables|/Script/UMG.Widget|SetRenderOpacity _output_get_2 0.0))))

(event EventInteract
  (bind _start_z (Variables|Default|GetStart%20Z))
  ;[0 1 1] simple interact event, can be changed for children
  (Audio|PlaySound2D "/Game/Sound/S_bloop_hover_3_.S_bloop_hover_3_" 1.0 (Math|Random|RandomFloatinRange 0.8 1.2) 0.0 0 0)
  (if (Variables|Default|GetOpen?)
    (Variables|Default|SetOpen? false)
    (bind _move (Timeline|Timeline Play)
      (:Update
        (Transformation|SetWorldRotation (Variables|Default|GetHinge) (Math|Rotator|MakeRotator 0.0 0.0 (Math|Float|Lerp _start_z (+ _start_z -9e+01) _move)) false false)))
    (else
      (Variables|Default|SetOpen? true)
      (Timeline|Timeline Reverse))))

(fn ConstructionScript)