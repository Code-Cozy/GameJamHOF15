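; Camera trigger volume that, depending on its Start flag, either begins a scripted pursuit camera shot or returns the view to the player.
; When the player enters a start trigger, it becomes the view target, sends an invert-controls message and runs a Timeline moving its Camera along a Spline.
; A non-start trigger blends back to the character and clears inversion.
; Timeline play rate is the reciprocal of Speed, so higher values mean slower movement.
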(event OnComponentBeginOverlap(Box)
  (params (OverlappedComponent :type Primitive%20Component%20Object%20Reference) (OtherActor :type Actor%20Object%20Reference) (OtherComp :type Primitive%20Component%20Object%20Reference) (OtherBodyIndex :type Integer) (bFromSweep :type Boolean) (SweepResult :type Hit%20Result%20Structure%20%28by%20ref%29))
  (bind _returnvalue (Game|GetPlayerCharacter 0))
  (if (== OtherActor (Game|GetPlayerCharacter 0))
    (if (Variables|Default|GetStart?)
      (Variables|Default|SetActive? true)
      (Game|Player|SetViewTargetwithBlend (Game|GetPlayerController 0) self 0.0 "VTBlend_Linear" 0.0 false)
      (CallFunction|Pursuit)
      (Class|BPIPlayer|InvertControlls(Message) (Game|GetPlayerCharacter 0) true)
      (else
        (Game|Player|SetViewTargetwithBlend (Game|GetPlayerController 0) _returnvalue 2.0 "VTBlend_Linear" 0.0 false)
        (Class|BPIPlayer|InvertControlls(Message) _returnvalue false)))))

(event Custom|Pursuit
  (bind _spline (Variables|Default|GetSpline))
  (bind _movement (Timeline|Timeline PlayFromStart)
    (:Update
      (Transformation|SetWorldLocation (Variables|Default|GetCamera) (Spline|GetLocationatDistanceAlongSpline (Variables|Default|GetSpline) (Math|Float|Lerp 0.0 (Spline|GetDistanceAlongSplineatSplinePoint _spline (- (Spline|GetNumberOfSplinePoints _spline) 1)) _movement) "World") false true))))

(event EventBeginPlay
  (Components|Timeline|SetPlayRate (Variables|Default|GetTimeline) (/ 1.0 (Variables|Default|GetSpeed))))

(fn ConstructionScript)