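; BP_Mimic is a chasing enemy that follows a spline path and sends the player to the menu map on contact.
; TriggerChase sends the player an invert-controls message and plays a timeline that teleports the skeletal mesh along the spline by distance.
; The Playrate variable acts as chase duration, since its reciprocal sets the timeline's play rate.
; Overlapping the box opens Map_Menu, while finishing the path only prints "survived".
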(event OnComponentBeginOverlap(Box)
  (params (OverlappedComponent :type Primitive%20Component%20Object%20Reference) (OtherActor :type Actor%20Object%20Reference) (OtherComp :type Primitive%20Component%20Object%20Reference) (OtherBodyIndex :type Integer) (bFromSweep :type Boolean) (SweepResult :type Hit%20Result%20Structure%20%28by%20ref%29))
  ;[0 1 1] trigger jumpscare
  (if (== OtherActor (Game|GetPlayerCharacter 0))
    (Game|OpenLevel(byObjectReference) "/Game/Maps/Map_Menu.Map_Menu")))

(event EventTriggerChase
  (bind _spline (Variables|Default|GetSpline))
  ;[0 1 1] movement of mimic
  (Class|BPIPlayer|InvertControlls(Message) (Game|GetPlayerCharacter 0) true)
  (bind _movement (Timeline|Timeline PlayFromStart)
    (:Update
      (Transformation|SetWorldLocation (Variables|Default|GetSkeletalMesh) (Spline|GetLocationatDistanceAlongSpline (Variables|Default|GetSpline) (Math|Float|Lerp 0.0 (Spline|GetDistanceAlongSplineatSplinePoint _spline (- (Spline|GetNumberOfSplinePoints _spline) 1)) _movement) "World") false true))
    (:Finished
      (Development|PrintString "survived" true true "(R=0.128440,G=1.000000,B=0.000000,A=1.000000)"))))

(event EventBeginPlay
  ;[0 1 1] set speed of movement on timeline
  (Components|Timeline|SetPlayRate (Variables|Default|GetTimeline) (/ 1.0 (Variables|Default|GetPlayrate))))

(fn ConstructionScript)