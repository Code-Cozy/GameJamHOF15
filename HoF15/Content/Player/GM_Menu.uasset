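; GM_Menu is the menu game mode, choosing between a splash screen and the main menu when play begins.
; If the Mushling game instance's FirstStartComplete is set, it spawns the menu and wakes the BP_Mushling_Menu actor.
; Otherwise it shows WBP_Splash, whose Done event triggers SpawnMenu, and writes the flag back unchanged.
; SpawnMenu creates WBP_Main only once, with UI-only input, a visible cursor and two 2D sounds.
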(event Custom|Spawn%20Menu
  (bind _returnvalue (Game|GetPlayerController 0))
  (Variables|Default|GetMenu
    (:then)
    (:else
      (bind _returnvalue_2 (UserInterface|CreateWidget "/Game/Widget/WBP_Main.WBP_Main_C"))
      (Variables|Default|SetMenu _returnvalue_2)
      (UserInterface|Viewport|AddtoPlayerScreen _returnvalue_2)
      (Input|SetInputModeUIOnly _returnvalue _returnvalue_2 "DoNotLock" true)
      (Variables|/Script/Engine.PlayerController|SetbShowMouseCursor _returnvalue true)
      (Audio|PlaySound2D "/Game/Sound/S_bloop_hover_3_.S_bloop_hover_3_" 1.0 1.0 0.0 0 0)
      (Audio|PlaySound2D "/Game/Sound/S_School.S_School" 1.0 1.0 0.0 0 0))))

(event EventBeginPlay
  (bind _returnvalue (Game|GetPlayerController 0))
  (bind _asgi_mushling (Utilities|Casting|CastToGI_Mushling (Game|GetGameInstance)))
  (if (Variables|/Game/Player/GI_Mushling.GI_Mushling_C|GetFirst%20Start%20Complete _asgi_mushling)
    (CallFunction|SpawnMenu)
    (bind _returnvalue_2 (Actor|GetActorOfClass "/Game/Player/BP_Mushling_Menu.BP_Mushling_Menu_C"))
    (Default|WakeUp _returnvalue_2)
    (else
      (Variables|/Game/Player/GI_Mushling.GI_Mushling_C|SetFirst%20Start%20Complete _asgi_mushling (Variables|/Game/Player/GI_Mushling.GI_Mushling_C|GetFirst%20Start%20Complete _asgi_mushling))
      (Input|SetInputModeUIOnly _returnvalue 0 "DoNotLock" false)
      (Variables|/Script/Engine.PlayerController|SetbShowMouseCursor _returnvalue true)
      (bind _returnvalue_3 (UserInterface|CreateWidget "/Game/Widget/WBP_Splash.WBP_Splash_C"))
      (UserInterface|Viewport|AddtoPlayerScreen _returnvalue_3)
      (EventDispatchers|BindEventtoDone _returnvalue_3 (delegate Custom|Spawn%20Menu)))))

(fn ConstructionScript)