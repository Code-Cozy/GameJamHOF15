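; BP_Mushling is the player character, handling movement, look, jump, sprint and pausing through Enhanced Input, with a clamped camera pitch.
; Interact sends a message to the currently registered Interactable, and three key flags feed a CheckKeys all-collected test.
; InvertControlls flips movement input and switches the view to a spawned camera on SpringArm1, later blending back to the character and destroying that camera.
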(event Input|EnhancedActionEvents|EnhancedInputActionIA_Pause
  (params (ActionValue :type Boolean) (ElapsedSeconds :type Float%20%28double-precision%29) (TriggeredSeconds :type Float%20%28double-precision%29) (InputAction :type Input%20Action%20Object%20Reference :default "/Game/Player/Input/IA_Pause.IA_Pause"))
  ;[0 1 1] pause game and spawn pause menu
  (:Triggered
    (Utilities|FlowControl|DoOnce false :!label _label
      (:Completed
        (if (Game|IsGamePaused)
          (Game|SetGamePaused false)
          (Widget|RemovefromParent (Variables|Default|GetPause%20Menu))
          (Variables|Default|SetPause%20Menu 0)
          (else
            (Game|SetGamePaused true)
            (bind _returnvalue (UserInterface|CreateWidget "/Game/Widget/WBP_Pause.WBP_Pause_C"))
            (Variables|Default|SetPause%20Menu _returnvalue)
            (UserInterface|Viewport|AddtoPlayerScreen _returnvalue))))))
  (:Completed
    (goto _label Reset)))

(event Input|EnhancedActionEvents|EnhancedInputActionIA_Jump
  (params (ActionValue :type Boolean) (ElapsedSeconds :type Float%20%28double-precision%29) (TriggeredSeconds :type Float%20%28double-precision%29) (InputAction :type Input%20Action%20Object%20Reference :default "/Game/Player/Input/IA_Jump.IA_Jump"))
  ;[0 1 1] jumping
  (:Started
    (Utilities|FlowControl|DoOnce false :!label _label
      (:Completed
        (Character|Jump))))
  (:Completed
    (Character|StopJumping)
    (goto _label Reset)))

(event Input|EnhancedActionEvents|EnhancedInputActionIA_Movement
  (params (ActionValue :type Vector%202D%20Structure) (ElapsedSeconds :type Float%20%28double-precision%29) (TriggeredSeconds :type Float%20%28double-precision%29) (InputAction :type Input%20Action%20Object%20Reference :default "/Game/Player/Input/IA_Movement.IA_Movement"))
  (bind _self self)
  (bind _self_2 self)
  (bind _returnvalue (Pawn|GetControlRotation _self :!class /Script/Engine.Pawn))
  (bind _returnvalue_2 (Pawn|GetControlRotation _self_2 :!class /Script/Engine.Pawn))
  (bind _returnvalue_3 (Math|Vector|GetRightVector (Math|Rotator|MakeRotator (.roll _returnvalue_2) 0.0 (.yaw _returnvalue_2))))
  (bind _returnvalue_4 (Math|Vector|GetForwardVector (Math|Rotator|MakeRotator 0.0 0.0 (.yaw _returnvalue))))
  ;[0 1 1] Movement
  (Utilities|FlowControl|Sequence
    (:then_0
      (if (Variables|Default|GetInvert)
        (Pawn|Input|AddMovementInput _returnvalue_3 (* (.x ActionValue) -1.0) false)
        (else
          (Pawn|Input|AddMovementInput _returnvalue_3 (.x ActionValue) false))))
    (:then_1
      (if (Variables|Default|GetInvert)
        (Pawn|Input|AddMovementInput _returnvalue_4 (* (.y ActionValue) -1.0) false)
        (else
          (Pawn|Input|AddMovementInput _returnvalue_4 (.y ActionValue) false))))))

(event Input|EnhancedActionEvents|EnhancedInputActionIA_Look
  (params (ActionValue :type Vector%202D%20Structure) (ElapsedSeconds :type Float%20%28double-precision%29) (TriggeredSeconds :type Float%20%28double-precision%29) (InputAction :type Input%20Action%20Object%20Reference :default "/Game/Player/Input/IA_Look.IA_Look"))
  ;[0 1 1] Mouse movement
  (Pawn|Input|AddControllerYawInput (.x ActionValue))
  (Pawn|Input|AddControllerPitchInput (* (.y ActionValue) -1.0)))

(event Input|EnhancedActionEvents|EnhancedInputActionIA_Sprint
  (params (ActionValue :type Boolean) (ElapsedSeconds :type Float%20%28double-precision%29) (TriggeredSeconds :type Float%20%28double-precision%29) (InputAction :type Input%20Action%20Object%20Reference :default "/Game/Player/Input/IA_Sprint.IA_Sprint"))
  (bind _charactermovement (Variables|Character|GetCharacterMovement))
  ;[0 1 1] sprinting speed
  (:Started
    (Variables|/Script/Engine.CharacterMovementComponent|SetMaxWalkSpeed _charactermovement 6e+02)
    (Variables|Default|SetSprint? true))
  (:Completed
    (Variables|/Script/Engine.CharacterMovementComponent|SetMaxWalkSpeed _charactermovement 3.5e+02)
    (Variables|Default|SetSprint? false)))

(event Input|EnhancedActionEvents|EnhancedInputActionIA_Interact
  (params (ActionValue :type Boolean) (ElapsedSeconds :type Float%20%28double-precision%29) (TriggeredSeconds :type Float%20%28double-precision%29) (InputAction :type Input%20Action%20Object%20Reference :default "/Game/Player/Input/IA_Interact.IA_Interact"))
  ;[0 1 1] Interact
  (:Triggered
    (Utilities|FlowControl|DoOnce false :!label _label
      (:Completed
        (bind _interactable (Variables|Default|GetInteractable)
          (:then
            (Class|BPIInteract|Interact(Message) _interactable))
          (:else)))))
  (:Completed
    (goto _label Reset)))

(event EventCloseWidget
  ;[0 1 1] pause game and spawn pause menu
  (Game|SetGamePaused false)
  (Widget|RemovefromParent (Variables|Default|GetPause%20Menu))
  (Variables|Default|SetPause%20Menu 0))

(event EventBeginPlay
  (bind _returnvalue (Game|GetPlayerCameraManager 0))
  ;[0 1 1] movement and camera lock
  (bind _aspc_mushling (Utilities|Casting|CastToPC_Mushling (Game|GetPlayerController 0)))
  (Variables|Default|SetMy%20Controller _aspc_mushling)
  (Variables|/Script/Engine.PlayerCameraManager|SetViewPitchMin _returnvalue -6e+01)
  (Variables|/Script/Engine.PlayerCameraManager|SetViewPitchMax _returnvalue 2e+01))

(event EventUpdateInteractable
  (params (Actor :type Actor%20Object%20Reference))
  ;[0 1 1] update interactable
  (Variables|Default|SetInteractable Actor))

(event EventGetKey
  (params (Int :type Integer))
  (switch int Int
    (:1
      (Variables|Default|SetKey1? true))
    (:2
      (Variables|Default|SetKey2? true))
    (:3
      (Variables|Default|SetKey3? true))))

(event EventInvertControlls
  (params (Invert :type Boolean))
  (bind _returnvalue (Game|GetPlayerController 0))
  (bind _output_get (Variables|Default|SetInvert Invert))
  (if _output_get
    (bind _returnvalue_2 (Game|SpawnActorfromClass "/Script/Engine.CameraActor" (Math|Transform|MakeTransform "0, 0, 0" "0, 0, 0" "1.000000,1.000000,1.000000") "AlwaysSpawn" "MultiplyWithRoot" 0 0))
    (bind _output_get_2 (Variables|Default|SetChase%20Camera _returnvalue_2))
    (Transformation|AttachComponentToComponent _output_get_2 (Variables|Default|GetSpringArm1) "None" "SnapToTarget" "SnapToTarget" "SnapToTarget" true)
    (Game|Player|SetViewTargetwithBlend _returnvalue _output_get_2 0.0 "VTBlend_Linear" 0.0 false)
    (Collision|SetActorEnableCollision _output_get_2 true)
    (else
      (Game|Player|SetViewTargetwithBlend _returnvalue (Game|GetPlayerCharacter 0) 1.0 "VTBlend_Linear" 0.0 false)
      (Utilities|FlowControl|Delay 1.0)
      (bind _chase_camera (Variables|Default|GetChase%20Camera)
        (:then
          (Actor|DestroyActor _chase_camera))
        (:else)))))

(fn ConstructionScript)

(fn CheckKeys
  (if (Variables|Default|GetKey1?)
    (if (Variables|Default|GetKey2?)
      (if (Variables|Default|GetKey3?)
        (return true)
        (else
          _))))
  (return false))