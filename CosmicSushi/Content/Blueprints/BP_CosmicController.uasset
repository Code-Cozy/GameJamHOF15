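; BP_CosmicController is a player controller that owns the game's HUD and switches it between menu and gameplay views.
; On BeginPlay it creates WBP_HUD, adds it to the viewport, enables Game and UI input and shows the mouse cursor.
; SwitchHUDView maps a HUD type to the widget switcher's active page.
; The Is At Edge graph holds only an unused screen-edge style threshold expression.
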(event EventBeginPlay
  (bind _returnvalue (UserInterface|CreateWidget "/Game/Widgets/WBP_HUD.WBP_HUD_C"))
  (bind _output_get (Variables|Default|SetHUD _returnvalue))
  (UserInterface|Viewport|AddtoViewport _output_get 0)
  (Input|SetInputModeGameandUI self _returnvalue "DoNotLock" true false)
  (Variables|Default|SetbShowMouseCursor true))

(event EventSwitchHUDView
  (params (HUD%20Type :type E_HUDView%20Enum :default "NewEnumerator0"))
  (bind _hud (Variables|Default|GetHUD))
  (bind _widgetswitcher (Variables|/Game/Widgets/WBP_HUD.WBP_HUD_C|GetWidgetSwitcher _hud))
  (switch Utilities|FlowControl|Switch|SwitchonE_HUDView HUD%20Type
    (:NewEnumerator0
      (Class|WidgetSwitcher|SetActiveWidgetIndex _widgetswitcher))
    (:NewEnumerator1
      (Class|WidgetSwitcher|SetActiveWidgetIndex _widgetswitcher 1))))

(fn ConstructionScript)