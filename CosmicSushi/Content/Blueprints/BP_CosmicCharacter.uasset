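; BP_CosmicCharacter is a pawn that pans across the world by screen-edge mouse scrolling.
; A Start interface call sets a flag that enables the scrolling.
; The MouseX and MouseY axis events compare the cursor position to the viewport edges within a threshold.
; Near an edge, the actor moves along world X or Y by a delta-time-scaled scroll speed, using teleported offsets.
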(event EventStart
  ;[0.15 0.15 0.15 0.5] bpi start call
  (Variables|Default|SetStart? true))

(event Input|MouseEvents|MouseX
  (params (AxisValue :type Float%20%28single-precision%29))
  (bind _returnvalue (Game|GetPlayerController 0))
  (bind _returnvalue_2 (Utilities|Time|GetWorldDeltaSeconds))
  (bind _threshold (Variables|Default|GetThreshold))
  (bind _scroll_speed (Variables|Default|GetScroll%20Speed))
  (bind _locationx (Game|Player|GetMousePosition _returnvalue))
  (bind _returnvalue_3 (* _scroll_speed _returnvalue_2))
  ;[0.15 0.15 0.15 0.5] edge border scrolling
  (if (Variables|Default|GetStart?)
    (Utilities|FlowControl|Sequence
      (:then_0
        (if (> _locationx (- (.x (Viewport|GetViewportSize)) _threshold)) ; Right
          (Transformation|AddActorWorldOffset (Math|Vector|MakeVector _returnvalue_3 0.0 0.0) false true)))
      (:then_1
        (if (< _locationx _threshold) ; Left
          (Transformation|AddActorWorldOffset (Math|Vector|MakeVector (* _returnvalue_3 -1.0) 0.0 0.0) false true))))))

(event Input|MouseEvents|MouseY
  (params (AxisValue :type Float%20%28single-precision%29))
  (bind _returnvalue (Utilities|Time|GetWorldDeltaSeconds))
  (bind _returnvalue_2 (Game|GetPlayerController 0))
  (bind _scroll_speed (Variables|Default|GetScroll%20Speed))
  (bind _threshold (Variables|Default|GetThreshold))
  (bind _locationy (Game|Player|GetMousePosition _returnvalue_2))
  (bind _returnvalue_3 (* _scroll_speed _returnvalue))
  ;[0.15 0.15 0.15 0.5] edge border scrolling
  (if (Variables|Default|GetStart?)
    (Utilities|FlowControl|Sequence
      (:then_0
        (if (> _locationy (- (.y (Viewport|GetViewportSize)) _threshold)) ; down
          (Transformation|AddActorWorldOffset (Math|Vector|MakeVector 0.0 _returnvalue_3 0.0) false true)))
      (:then_1
        (if (< _locationy _threshold) ; up
          (Transformation|AddActorWorldOffset (Math|Vector|MakeVector 0.0 (* _returnvalue_3 -1.0) 0.0) false true))))))

(fn ConstructionScript)